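; BP_Projectile is a projectile that destroys enemies and awards the player a point per kill.
; Mesh overlap with BP_Enemy increments PlayerScore, destroys both actors and plays an explosion sound, while overlapping BP_Tunnel destroys only the projectile.
; Any hit also destroys it, and an end overlap with another BP_Projectile destroys that other one.
; Tick repeatedly adds a score-scaled amount to ProjectileMovement's InitialSpeed, without setting Velocity.
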(event `self.ProjectileMesh.OnComponentBeginOverlap`
  (params (OverlappedComponent :type "PrimitiveComponent Object Reference") (OtherActor :type "Actor Object Reference") (OtherComp :type "PrimitiveComponent Object Reference") (OtherBodyIndex :type Integer) (bFromSweep :type Boolean) (SweepResult :type "HitResult Structure (by ref)"))
  (bind _asbp_enemy (cast `/Game/InfiniteMatrix/Blueprints/BP_Enemy` OtherActor)
    (:`then`
      (bind _asbp_player (cast `/Game/InfiniteMatrix/Blueprints/BP_Player` (`GameplayStatics.GetPlayerPawn` 0)))
      (set `/Game/InfiniteMatrix/Blueprints/BP_Player.PlayerScore` (+ (`/Game/InfiniteMatrix/Blueprints/BP_Player.PlayerScore` _asbp_player) 1) _asbp_player)
      (`self.K2_DestroyActor` _asbp_enemy)
      (`self.K2_DestroyActor`)
      (`GameplayStatics.PlaySound2D` "/Game/InfiniteMatrix/Sounds/explosionCrunch_000.explosionCrunch_000" 1.0 1.0 0.0 null null))
    (:`CastFailed`
      (cast `/Game/InfiniteMatrix/Blueprints/BP_Tunnel` OtherActor)
      (`self.K2_DestroyActor`))))

(event `self.ProjectileMesh.OnComponentEndOverlap`
  (params (OverlappedComponent :type "PrimitiveComponent Object Reference") (OtherActor :type "Actor Object Reference") (OtherComp :type "PrimitiveComponent Object Reference") (OtherBodyIndex :type Integer))
  (bind _asbp_projectile (cast `/Game/InfiniteMatrix/Blueprints/BP_Projectile` OtherActor))
  (`self.K2_DestroyActor` _asbp_projectile))

(event `self.ProjectileMesh.OnComponentHit`
  (params (HitComponent :type "PrimitiveComponent Object Reference") (OtherActor :type "Actor Object Reference") (OtherComp :type "PrimitiveComponent Object Reference") (NormalImpulse :type "Vector Structure") (Hit :type "HitResult Structure (by ref)"))
  (`self.K2_DestroyActor`))

(event `self.ReceiveTick`
  (params (DeltaSeconds :type "Float (single-precision)"))
  (bind _projectilemovement (`self.ProjectileMovement`))
  (bind _asbp_player (cast `/Game/InfiniteMatrix/Blueprints/BP_Player` (`GameplayStatics.GetPlayerPawn` 0)))
  (set `ProjectileMovementComponent.InitialSpeed` (+ (`ProjectileMovementComponent.InitialSpeed` _projectilemovement) (* (`/Game/InfiniteMatrix/Blueprints/BP_Player.PlayerScore` _asbp_player) 30)) _projectilemovement))

(fn `UserConstructionScript`)