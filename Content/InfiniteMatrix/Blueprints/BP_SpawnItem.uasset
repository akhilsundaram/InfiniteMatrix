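; BP_SpawnItem is a spawner for health packs and enemies placed ahead of the player, currently inactive.
; RandomLocationFromActor picks a random point at an X offset from the player pawn, with Y and Z in fixed world ranges.
; SpawnHealthpack and SpawnEnemy spawn BP_health and BP_Enemy at given locations.
; BeginPlay and Spawner are empty; the delayed spawn loop and the paired spawn calls are disconnected, so nothing spawns.
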(event `self.ReceiveBeginPlay`)

(fn `RandomLocationFromActor`
  (returns (`x-component` :type "Float (double-precision)") (`y-component` :type "Float (double-precision)") (`z-component` :type "Float (double-precision)"))
  (bind _returnvalue_x (`KismetMathLibrary.BreakVector` (`self.K2_GetActorLocation` (`GameplayStatics.GetPlayerPawn` 0))))
  (return (+ _returnvalue_x (`KismetMathLibrary.RandomIntegerInRange` 1000 3000)) (`KismetMathLibrary.Conv_IntToDouble` (`KismetMathLibrary.RandomIntegerInRange` 0 700)) (`KismetMathLibrary.Conv_IntToDouble` (`KismetMathLibrary.RandomIntegerInRange` 0 700))))

(fn `SpawnEnemy`
  (params (SpawnLocation :type "Vector Structure"))
  (`|SpawnActorFromClass` "/Game/InfiniteMatrix/Blueprints/BP_Enemy.BP_Enemy_C" (`KismetMathLibrary.MakeTransform` SpawnLocation) "Undefined" "MultiplyWithRoot" null null))

(fn `Spawner`)

(fn `SpawnHealthpack`
  (params (SpawnLocation :type "Vector Structure"))
  (`|SpawnActorFromClass` "/Game/InfiniteMatrix/Blueprints/BP_health.BP_health_C" (`KismetMathLibrary.MakeTransform` SpawnLocation) "Undefined" "MultiplyWithRoot" null null))

(fn `UserConstructionScript`)