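; BP_health is a rotating food pickup that restores one point of player health on overlap, with health capped around ten.
; FoodMesh spins on yaw each tick at RotateSpeed.
; An overlap by BP_Player raises PlayerHealth, refreshes the widget text through the NewHUD UI reference, and plays a sound, even at full health.
; The actor is not destroyed or disabled afterwards, so each new overlap triggers it again.
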(event `self.FoodMesh.OnComponentBeginOverlap`
  (params (OverlappedComponent :type "PrimitiveComponent Object Reference") (OtherActor :type "Actor Object Reference") (OtherComp :type "PrimitiveComponent Object Reference") (OtherBodyIndex :type Integer) (bFromSweep :type Boolean) (SweepResult :type "HitResult Structure (by ref)"))
  (bind _asbp_player (cast `/Game/InfiniteMatrix/Blueprints/BP_Player` OtherActor))
  (bind _playerhealth (`/Game/InfiniteMatrix/Blueprints/BP_Player.PlayerHealth` _asbp_player))
  (if (<= _playerhealth 9)
    (set `/Game/InfiniteMatrix/Blueprints/BP_Player.PlayerHealth` (+ _playerhealth 1) _asbp_player))
  (`self.UpdateHUD`)
  (`GameplayStatics.PlaySound2D` "/Game/InfiniteMatrix/Sounds/impactMining_000.impactMining_000" 1.0 1.0 0.0 null null))

(event `self.ReceiveTick`
  (params (DeltaSeconds :type "Float (single-precision)"))
  (`SceneComponent.K2_AddLocalRotation` (`self.FoodMesh`) (`KismetMathLibrary.MakeRotator` 0.0 0.0 (* DeltaSeconds (`self.RotateSpeed`))) false false))

(fn `UpdateHUD`
  (bind _asnew_hud (cast `/Game/Blueprints/NewHUD` (`PlayerController.GetHUD` (`GameplayStatics.GetPlayerController` 0))))
  (`/Game/Score_widget.UpdateWidgetText` (`/Game/Blueprints/NewHUD.UIRef` _asnew_hud)))

(fn `UserConstructionScript`)